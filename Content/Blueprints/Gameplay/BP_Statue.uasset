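; BP_Statue is a statue actor that highlights and becomes physical while the main character is near it.
; Sphere overlap events, filtered to BP_MainCharacter, drive its static mesh.
; On entry the mesh gains an outline overlay material, physics simulation and query-and-physics collision.
; On exit it clears the overlay, stops simulating and disables collision entirely.
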(event OnComponentBeginOverlap(Sphere)
  (params (OverlappedComponent :type Primitive%20Component%20Object%20Reference) (OtherActor :type Actor%20Object%20Reference) (OtherComp :type Primitive%20Component%20Object%20Reference) (OtherBodyIndex :type Integer) (bFromSweep :type Boolean) (SweepResult :type Hit%20Result%20Structure%20%28by%20ref%29))
  (bind _staticmesh (Variables|Default|GetStaticMesh))
  (Utilities|Casting|CastToBP_MainCharacter OtherActor)
  (Rendering|Material|SetOverlayMaterial _staticmesh "/Game/Assets/Materials/M_Outline_Inst.M_Outline_Inst" :!class /Script/Engine.MeshComponent)
  (Physics|SetSimulatePhysics _staticmesh true)
  (Collision|SetCollisionEnabled _staticmesh "QueryAndPhysics"))

(event OnComponentEndOverlap(Sphere)
  (params (OverlappedComponent :type Primitive%20Component%20Object%20Reference) (OtherActor :type Actor%20Object%20Reference) (OtherComp :type Primitive%20Component%20Object%20Reference) (OtherBodyIndex :type Integer))
  (bind _staticmesh (Variables|Default|GetStaticMesh))
  (Utilities|Casting|CastToBP_MainCharacter OtherActor)
  (Rendering|Material|SetOverlayMaterial (Variables|Default|GetStaticMesh) 0 :!class /Script/Engine.MeshComponent)
  (Physics|SetSimulatePhysics _staticmesh false)
  (Collision|SetCollisionEnabled _staticmesh "NoCollision"))

(fn ConstructionScript)