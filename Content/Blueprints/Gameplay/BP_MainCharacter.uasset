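; BP_MainCharacter is the main character Blueprint, which emits movement noise for AI hearing.
; Each tick with non-zero velocity, it picks a loudness from its movement state: loudest when running, quietest when crouching, in between otherwise.
; It then reports a noise event at the actor's location with itself as instigator and a short fixed max range.
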(event EventTick
  (params (DeltaSeconds :type Float%20%28single-precision%29))
  (if (!= (Math|Vector|VectorLength (Transformation|GetVelocity)) 0.0)
    (bind _returnvalue (Class|MainCharacter|IsRunning))
    (if _returnvalue
      (Variables|Default|SetLoudness 3e+02)
      (else
        (bind _returnvalue_2 (Class|MainCharacter|IsCrouching))
        (if _returnvalue_2
          (Variables|Default|SetLoudness 3e+01)
          (else
            (Variables|Default|SetLoudness 1e+02)))))
    (Class|AISenseHearing|ReportNoiseEvent (Transformation|GetActorLocation) (Variables|Default|GetLoudness) self 1e+01 "None")))

(fn ConstructionScript)